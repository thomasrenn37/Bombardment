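; BP_MyCharacter is a basic player character Blueprint that handles movement, looking and jumping from input mappings.
; Forward/back and left/right axes feed AddMovementInput along the actor's forward and right vectors, while look axes drive controller yaw and pitch.
; The Jump action calls Jump on press and StopJumping on release, and the construction script is empty.
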(event `InputAxis|Move_Forward_Backward`
  (params (AxisValue :type "Float (single-precision)"))
  ;[1 1 1] Player Movement
  (`self.AddMovementInput` (`self.GetActorForwardVector`) AxisValue))

(event `InputAction|Jump`
  (params (Key :type "Key Structure"))
  ;[1 1 1] Jumping Action
  (:`Pressed`
    (`self.Jump`))
  (:`Released`
    (`self.StopJumping`)))

(event `InputAxis|Move_Left_Right`
  (params (AxisValue :type "Float (single-precision)"))
  ;[1 1 1] Player Movement
  (`self.AddMovementInput` (`self.GetActorRightVector`) AxisValue))

(event `InputAxis|Look_Left_Right`
  (params (AxisValue :type "Float (single-precision)"))
  ;[1 1 1] Player Look // Yaw and pitch
  (`self.AddControllerYawInput` AxisValue))

(event `InputAxis|Look_Up_Down`
  (params (AxisValue :type "Float (single-precision)"))
  ;[1 1 1] Player Look // Yaw and pitch
  (`self.AddControllerPitchInput` AxisValue))

(fn `UserConstructionScript`)