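; Grenade Blueprint for a timed explosive that detonates after a delay from BeginPlay.
; On detonation it damages Player-class actors overlapping its sphere and fires a radial force impulse.
; It then stops and hides the mesh, activates the explosion effect, plays a sound at world origin, and destroys itself after a short delay.
; Activation of the radial force component also fires an impulse.
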(event `self.ReceiveBeginPlay`
  (bind _throwablestaticmesh (`self.ThrowableStaticMesh`))
  (`KismetSystemLibrary.Delay` (`self.delayTime`))
  (for _array_element (`PrimitiveComponent.GetOverlappingActors` (`self.Sphere`) "/Game/Blueprints/Characters/Player.Player_C")
    (`GameplayStatics.ApplyDamage` _array_element 50.0 null self))
  (`RadialForceComponent.FireImpulse` (`self.RadForce`))
  (`PrimitiveComponent.SetSimulatePhysics` _throwablestaticmesh false)
  (`SceneComponent.SetVisibility` _throwablestaticmesh false false)
  (`ActorComponent.Activate` (`self.Explosion`) true)
  (`GameplayStatics.PlaySoundAtLocation` "/Game/StarterContent/Audio/Explosion02.Explosion02" (0.0 0.0 0.0) (struct) 1.0 1.0 0.0 null null null null)
  (`KismetSystemLibrary.Delay` 3.0)
  (`self.K2_DestroyActor`))

(event `self.RadForce.OnComponentActivated`
  (params (Component :type "ActorComponent Object Reference") (bReset :type Boolean))
  (`RadialForceComponent.FireImpulse` (`self.RadForce`)))

(fn `UserConstructionScript`)