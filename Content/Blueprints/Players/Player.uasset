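; Player Blueprint that opens the pause menu when P is pressed.
; It creates and caches a PauseMenu widget on first use, then shows the mouse cursor, switches input to UI-only focused on the menu and adds it to the viewport.
; It then pauses the game, and the file has no unpause logic of its own.
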(event `Key|P`
  (params (Key :type "Key Structure"))
  (bind _pause_menu_reference (`self.Pause Menu Reference`))
  (bind _returnvalue (`PlayerState.GetPlayerController` (`GameplayStatics.GetPlayerState` 0)))
  (:`Pressed`
    (`/Engine/EditorBlueprintResources/StandardMacros.IsValid` (`self.Pause Menu Reference`)
      (:`Is Valid`
        _)
      (:`Is Not Valid`
        (bind _returnvalue_2 (`|CreateWidget` "/Game/UI/PauseMenu.PauseMenu_C"))
        (set `self.Pause Menu Reference` _returnvalue_2)))
    (set `PlayerController.bShowMouseCursor` true _returnvalue)
    (`WidgetBlueprintLibrary.SetInputMode_UIOnlyEx` _returnvalue _pause_menu_reference)
    (`UserWidget.AddToViewport` _pause_menu_reference 0)
    (`GameplayStatics.SetGamePaused` true)))

(fn `UserConstructionScript`)